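; BP_SaveGameManager is an actor that saves player progress, currently the sprint upgrade, to a fixed save slot.
; SaveGameData creates a fresh BP_SaveGame, copies CanSprint from the player's BP_ThirdPersonCharacter into HasSprintUpgrade, writes the slot and prints a confirmation.
; LoadGameData reads the same slot but does nothing with the result, so the upgrade is never restored here.
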(event `Save Game Data`
  (bind _returnvalue (`GameplayStatics.CreateSaveGameObject` "/Game/Blueprints/SaveLoadSystem/BP_SaveGame.BP_SaveGame_C"))
  (bind _output_get (set `self.saveGameRef` _returnvalue))
  (bind _asbp_third_person_character (cast `/Game/ThirdPerson/Blueprints/BP_ThirdPersonCharacter` (`GameplayStatics.GetPlayerCharacter` 0)))
  (set `/Game/Blueprints/SaveLoadSystem/BP_SaveGame.hasSprintUpgrade` (`/Game/ThirdPerson/Blueprints/BP_ThirdPersonCharacter.canSprint?` _asbp_third_person_character) _output_get)
  (`GameplayStatics.SaveGameToSlot` (`self.saveGameRef`) "PlayerSaveSlot")
  (`KismetSystemLibrary.PrintString` "Data saved!"))

(event `Load Game Data`
  (`GameplayStatics.LoadGameFromSlot` "PlayerSaveSlot"))

(fn `UserConstructionScript`)