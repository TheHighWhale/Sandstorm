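; Game mode that runs a sandstorm countdown and kills the player when it runs out.
; StartCountdown resets the timer and shows the WBP_SandstormTimer widget, then UpdateTimer re-calls itself after one-second delays, decrementing until zero.
; If InBase is true while time remains, the loop stops.
; At zero, StormEvent prints a warning, fades the camera to a sandy yellow and calls Death on the third-person character.
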(event `self.ReceiveBeginPlay`)

(event `Start Countdown`
  ;[1 1 1] Start Timer
  (set `self.CountdownTimer` 10)
  (bind _returnvalue (`|CreateWidget` "/Game/Blueprints/UI/WBP_SandstormTimer.WBP_SandstormTimer_C"))
  (`UserWidget.AddToViewport` _returnvalue 0)
  (`self.Update Timer`))

(event `Update Timer`
  ;[1 1 1] Timer
  (`KismetSystemLibrary.Delay` 1.0)
  (if (<= (`self.CountdownTimer`) 0)
    (`self.Storm Event`)
    (elif (not (`self.inBase?`))
      (set `self.CountdownTimer` (- (`self.CountdownTimer`) 1))
      (`self.Update Timer`))))

(event `Storm Event`
  ;[1 1 1] Storm Event and Respawn
  (`KismetSystemLibrary.PrintString` "Overwhelmed by the storm!")
  (`PlayerCameraManager.StartCameraFade` (`GameplayStatics.GetPlayerCameraManager` 0) 0.0 1.0 2.0 (struct :`R` 0.697917 :`G` 0.676211 :`B` 0.063187 :`A` 1.0) false false)
  (`KismetSystemLibrary.Delay` 1.9)
  (bind _asbp_third_person_character (cast `/Game/Blueprints/Player/BP_ThirdPersonCharacter` (`GameplayStatics.GetPlayerPawn` 0)))
  (`/Game/Blueprints/Player/BP_ThirdPersonCharacter.Death` _asbp_third_person_character))

(fn `UserConstructionScript`)